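; EnemyBP is a platformer enemy that walks back and forth horizontally.
; Tick feeds the current Direction into AddMovementInput for constant movement.
; A capsule component hit calls ChangeDirection, whose FlipFlop alternates Direction along the X axis and rotates the sprite to match.
; The hit handler does not filter what was struck, so every hit event triggers a turn.
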(event `self.ReceiveTick`
  (params (DeltaSeconds :type "Float (single-precision)"))
  (`self.AddMovementInput` (`self.Direction`)))

(event `ChangeDirection`
  (bind _sprite (`self.Sprite`))
  (`/Engine/EditorBlueprintResources/StandardMacros.FlipFlop`
    (:`A`
      (`SceneComponent.K2_SetWorldRotation` _sprite (struct :`Yaw` -180.0) false false)
      (set `self.Direction` (-1.0 0.0 0.0)))
    (:`B`
      (`SceneComponent.K2_SetWorldRotation` :`self` _sprite)
      (set `self.Direction` (1.0 0.0 0.0)))))

(event `self.CapsuleComponent.OnComponentHit`
  (params (HitComponent :type "PrimitiveComponent Object Reference") (OtherActor :type "Actor Object Reference") (OtherComp :type "PrimitiveComponent Object Reference") (NormalImpulse :type "Vector Structure") (Hit :type "HitResult Structure (by ref)"))
  (`self.ChangeDirection`))

(fn `UserConstructionScript`)