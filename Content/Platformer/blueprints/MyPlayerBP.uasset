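; Player character Blueprint for a 2D side-scrolling platformer, handling movement, jumping and death, and showing the score HUD on BeginPlay.
; Input moves it along world X and mirrors the flipbook sprite through negative X scale, with movement and jumping blocked once dead.
; A capsule hit from an "enemy"-tagged actor triggers death once, detaching the camera, playing the death flipbook, then showing the game-over widget and cursor after a delay.
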(event `self.ReceiveBeginPlay`
  (bind _returnvalue (`|CreateWidget` "/Game/Platformer/blueprints/ScoreWB.ScoreWB_C"))
  (bind _output_get (set `self.ScoreHUD` _returnvalue))
  (`UserWidget.AddToViewport` _output_get 0))

(event `InputAxis|Move`
  (params (AxisValue :type "Float (single-precision)"))
  (bind _sprite (`self.Sprite`))
  (if (not (`self.Dead`))
    (`self.AddMovementInput` (1.0 0.0 0.0) AxisValue)
    (`/Engine/EditorBlueprintResources/StandardMacros.CompareFloat` AxisValue
      (:`>`
        (`SceneComponent.SetRelativeScale3D` _sprite (0.5 0.5 0.5)))
      (:`<`
        (`SceneComponent.SetRelativeScale3D` _sprite (-0.5 0.5 0.5))))))

(event `InputAction|Jump`
  (params (Key :type "Key Structure"))
  (:`Pressed`
    (if (not (`self.Dead`))
      (`self.Jump`)))
  (:`Released`
    (`self.StopJumping`)))

(event `self.CapsuleComponent.OnComponentHit`
  (params (HitComponent :type "PrimitiveComponent Object Reference") (OtherActor :type "Actor Object Reference") (OtherComp :type "PrimitiveComponent Object Reference") (NormalImpulse :type "Vector Structure") (Hit :type "HitResult Structure (by ref)"))
  (bind _returnvalue (`GameplayStatics.GetPlayerController` 0))
  (bind _sprite (`self.Sprite`))
  (if (`self.ActorHasTag` OtherActor "enemy")
    (`/Engine/EditorBlueprintResources/StandardMacros.DoOnce` false
      (:`Completed`
        (set `self.Dead` true)
        (`SceneComponent.K2_AddLocalOffset` (`self.Sprite`) (0.0 0.0 -5.0) false false)
        (`SceneComponent.K2_DetachFromComponent` (`self.Camera`) "KeepWorld" "KeepWorld" "KeepWorld" true)
        (`PaperFlipbookComponent.SetLooping` _sprite false)
        (`PaperFlipbookComponent.SetFlipbook` _sprite "/Game/Platformer/sprites/OG_Player/DEATH.DEATH")
        (`KismetSystemLibrary.Delay` 2.0)
        (bind _returnvalue_2 (`|CreateWidget` "/Game/Platformer/levels/GameOverWB.GameOverWB_C" _returnvalue))
        (`UserWidget.AddToViewport` _returnvalue_2 0)
        (set `PlayerController.bShowMouseCursor` true _returnvalue)))))

(fn `UserConstructionScript`)